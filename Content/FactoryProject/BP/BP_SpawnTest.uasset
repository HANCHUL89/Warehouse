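; BP_SpawnTest is a test actor that rides along a conveyor spline like an item on a belt.
; On BeginPlay it finds a BP_ConveyorSpline actor in the level via GetActorOfClass.
; Each Tick it advances a distance by MoveSpeed, places its static mesh at that spline point with world-space location but local-space rotation, and destroys itself upon reaching the spline's end.
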(event `self.ReceiveBeginPlay`
  (bind _returnvalue (`GameplayStatics.GetActorOfClass` "/Game/FactoryProject/BP/BP_ConveyorSpline.BP_ConveyorSpline_C"))
  (set `self.ConveyorSpline` _returnvalue)
  (set `self.Distance` 0.0))

(event `self.ReceiveTick`
  (params (DeltaSeconds :type "Float (single-precision)"))
  (bind _conveyorspline (`/Game/FactoryProject/BP/BP_ConveyorSpline.ConveyorSpline` (`self.ConveyorSpline`)))
  (if (`KismetSystemLibrary.IsValid` (`self.ConveyorSpline`))
    (bind _output_get (set `self.Distance` (+ (* DeltaSeconds (`self.MoveSpeed`)) (`self.Distance`))))
    (`SceneComponent.K2_SetWorldLocationAndRotation` (`self.StaticMesh`) (`SplineComponent.GetLocationAtDistanceAlongSpline` _conveyorspline _output_get "World") (`SplineComponent.GetRotationAtDistanceAlongSpline` _conveyorspline _output_get "Local") false false)
    (if (>= (`self.Distance`) (`SplineComponent.GetSplineLength` (`/Game/FactoryProject/BP/BP_ConveyorSpline.ConveyorSpline` (`self.ConveyorSpline`))))
      (`self.K2_DestroyActor`))))

(fn `UserConstructionScript`)