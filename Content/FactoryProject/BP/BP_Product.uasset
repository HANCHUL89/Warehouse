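; BP_Product is a factory product whose static mesh rides along the conveyor spline found in the level at BeginPlay.
; Each Tick advances a distance by MoveSpeed and places the mesh at that spline point, using world-space location but local-space rotation.
; Reaching the spline's end sets a stop flag, which a timer clears after StopDuration; the distance is never reset, so the stop re-triggers.
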(event `self.ReceiveBeginPlay`
  (bind _returnvalue (`GameplayStatics.GetActorOfClass` "/Game/FactoryProject/BP/BP_ConveyorSpline.BP_ConveyorSpline_C"))
  (set `self.ConveyorSpline` _returnvalue))

(event `self.ReceiveTick`
  (params (DeltaSeconds :type "Float (single-precision)"))
  (`self.UpdateStopState` DeltaSeconds)
  (if (not (`self.Isstop`))
    (`self.MoveSpline` DeltaSeconds)
    (if (>= (`self.Distance`) (`SplineComponent.GetSplineLength` (`/Game/FactoryProject/BP/BP_ConveyorSpline.ConveyorSpline` (`self.ConveyorSpline`))))
      (set `self.Isstop` true))))

(fn `MoveSpline`
  (params (A :type "Float (double-precision)"))
  (bind _conveyorspline (`/Game/FactoryProject/BP/BP_ConveyorSpline.ConveyorSpline` (`self.ConveyorSpline`)))
  (if (`KismetSystemLibrary.IsValid` (`self.ConveyorSpline`))
    (bind _output_get (set `self.Distance` (+ (* A (`self.MoveSpeed`)) (`self.Distance`))))
    (`SceneComponent.K2_SetWorldLocationAndRotation` (`self.StaticMesh`) (`SplineComponent.GetLocationAtDistanceAlongSpline` _conveyorspline _output_get "World") (`SplineComponent.GetRotationAtDistanceAlongSpline` _conveyorspline _output_get "Local") false false)))

(fn `UpdateStopState`
  (params (DeltaSeconds :type "Float (double-precision)"))
  (if (`self.Isstop`)
    (set `self.StopTimer` (+ DeltaSeconds (`self.StopTimer`)))
    (if (>= (`self.StopTimer`) (`self.StopDuration`))
      (set `self.Isstop` false)
      (set `self.StopTimer` 0.0))))

(fn `UserConstructionScript`)