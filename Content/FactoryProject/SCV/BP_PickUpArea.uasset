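; BP_PickUpArea is a pick-up zone in the factory project that reports the BP_Product boxes inside its Area component.
; IsBoxInArea returns whether any product overlaps the Area.
; GetNearestBox loops over the overlapping products and returns the one closest to a given start location, using a running minimum distance.
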(fn `GetNearestBox`
  (params (StartLocation :type "Vector Structure"))
  (returns (NearestActor1 :type "Actor Object Reference"))
  (locals (NearestDist :type "Float (double-precision)" :default 99999.0) (NearestActor :type "Actor Object Reference"))
  (for _array_element (`PrimitiveComponent.GetOverlappingActors` (`self.Area`) "/Game/FactoryProject/BP/BP_Product.BP_Product_C")
    (bind _returnvalue (`KismetMathLibrary.Vector_Distance` (`self.K2_GetActorLocation` _array_element) (`local.StartLocation`)))
    (if (> (`local.NearestDist`) _returnvalue)
      (set `local.NearestDist` _returnvalue)
      (set `local.NearestActor` _array_element)))
  (return (`local.NearestActor`)))

(fn `IsBoxInArea`
  (returns (`In Box` :type Boolean))
  (return (`KismetArrayLibrary.Array_IsNotEmpty` (`PrimitiveComponent.GetOverlappingActors` (`self.Area`) "/Game/FactoryProject/BP/BP_Product.BP_Product_C"))))

(fn `UserConstructionScript`)