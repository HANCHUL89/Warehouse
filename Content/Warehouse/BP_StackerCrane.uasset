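; Warehouse stacker crane that stores pallets into and retrieves them from rack slots supplied by the pallet rack.
; Tick runs inbound or outbound state machines, using direction maps to move crane, lift and fork roots with clamped steps, flipping fork direction for odd slot indices.
; A pallet touching the fork is destroyed and represented by toggling a mesh's visibility.
; Rack occupancy updates during transfers, and inbound completion notifies the InboundManager.
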(event `self.ReceiveBeginPlay`
  (set `self.Jobtype` "NewEnumerator0")
  (`SceneComponent.SetVisibility` (`self.SM_Pallet`) false false))

(event `self.ForkCollision.OnComponentBeginOverlap`
  (params (OverlappedComponent :type "PrimitiveComponent Object Reference") (OtherActor :type "Actor Object Reference") (OtherComp :type "PrimitiveComponent Object Reference") (OtherBodyIndex :type Integer) (bFromSweep :type Boolean) (SweepResult :type "HitResult Structure (by ref)"))
  (bind _asbp_pallet (cast `/Game/Warehouse/BP_Pallet` OtherActor))
  (`self.K2_DestroyActor` _asbp_pallet)
  (`SceneComponent.SetVisibility` (`self.SM_Pallet`) true false))

(event `self.ReceiveTick`
  (params (DeltaSeconds :type "Float (single-precision)"))
  (bind (_value _returnvalue) (`BlueprintMapLibrary.Map_Find` (`self.MoveDirectionMap_Outbound`) (`self.OutboundMoveType`)))
  (bind (_value_2 _returnvalue_2) (`BlueprintMapLibrary.Map_Find` (`self.MoveDirectionMap_Inbound`) (`self.InboundMoveType`)))
  (bind (_relativelocation_x _relativelocation_y) (`KismetMathLibrary.BreakVector` (`SceneComponent.RelativeLocation` (`self.ForkRoot`))))
  (bind (_relativelocation_x_2 _relativelocation_y_2) (`KismetMathLibrary.BreakVector` (`SceneComponent.RelativeLocation` (`self.ForkRoot`))))
  (bind _relativelocation_x_3 (`KismetMathLibrary.BreakVector` (`SceneComponent.RelativeLocation` (`self.CraneRoot`))))
  (bind (_relativelocation_x_4 _relativelocation_y_3 _relativelocation_z) (`KismetMathLibrary.BreakVector` (`SceneComponent.RelativeLocation` (`self.LiftRoot`))))
  (bind (_relativelocation_x_5 _relativelocation_y_4) (`KismetMathLibrary.BreakVector` (`SceneComponent.RelativeLocation` (`self.ForkRoot`))))
  (bind _relativelocation_x_6 (`KismetMathLibrary.BreakVector` (`SceneComponent.RelativeLocation` (`self.CraneRoot`))))
  (bind (_relativelocation_x_7 _relativelocation_y_5) (`KismetMathLibrary.BreakVector` (`SceneComponent.RelativeLocation` (`self.ForkRoot`))))
  (bind (_relativelocation_x_8 _relativelocation_y_6) (`KismetMathLibrary.BreakVector` (`SceneComponent.RelativeLocation` (`self.ForkRoot`))))
  (bind (_relativelocation_x_9 _relativelocation_y_7 _relativelocation_z_2) (`KismetMathLibrary.BreakVector` (`SceneComponent.RelativeLocation` (`self.LiftRoot`))))
  (bind _relativelocation_x_10 (`KismetMathLibrary.BreakVector` (`SceneComponent.RelativeLocation` (`self.CraneRoot`))))
  (bind (_relativelocation_x_11 _relativelocation_y_8 _relativelocation_z_3) (`KismetMathLibrary.BreakVector` (`SceneComponent.RelativeLocation` (`self.LiftRoot`))))
  (bind (_relativelocation_x_12 _relativelocation_y_9) (`KismetMathLibrary.BreakVector` (`SceneComponent.RelativeLocation` (`self.ForkRoot`))))
  (bind (_craneaxis _liftaxis _forkaxis) (break `/Game/Warehouse/ST_MoveAxis` _value))
  (bind (_craneaxis_2 _liftaxis_2 _forkaxis_2) (break `/Game/Warehouse/ST_MoveAxis` _value_2))
  (switch `/Game/Warehouse/ENUM/EN_CraneJobType` (`self.Jobtype`)
    (:`NewEnumerator1`
      (if _returnvalue_2
        (`self.MoveAlongAxis` _craneaxis_2 (`self.CraneRoot`))
        (`self.MoveAlongAxis` _liftaxis_2 (`self.LiftRoot`))
        (`self.MoveAlongAxis` (* _forkaxis_2 (`self.ForkAxis`)) (`self.ForkRoot`))
        (`self.InboundDirectionMap`)))
    (:`NewEnumerator2`
      (if _returnvalue
        (`self.MoveAlongAxis` _craneaxis (`self.CraneRoot`))
        (`self.MoveAlongAxis` _liftaxis (`self.LiftRoot`))
        (`self.MoveAlongAxis` (* _forkaxis (`self.ForkAxis`)) (`self.ForkRoot`))
        (switch `/Game/Warehouse/ENUM/EN_OutboundMoveType` (`self.OutboundMoveType`)
          (:`NewEnumerator0`
            (set `self.Jobtype` "NewEnumerator0"))
          (:`NewEnumerator1`
            (if (>= _relativelocation_x_3 (* (`self.X`) 250))
              (if (>= _relativelocation_z (* (`self.Z`) 250))
                (set `self.OutboundMoveType` "NewEnumerator2"))))
          (:`NewEnumerator2`
            (if (== (mod (`self.Index`) 2) 0)
              (if (>= _relativelocation_y 250.0)
                (set `self.OutboundMoveType` "NewEnumerator3")
                (`SceneComponent.SetVisibility` (`self.SM_Pallet`) true false)
                (`/Game/Warehouse/BP_StorageSlot.SetSlotFull` (`self.PalleRack`) (`self.Index`) false))
              (else
                (set `self.ForkAxis` (0.0 -1.0 0.0))
                (if (<= _relativelocation_y_2 -250.0)
                  (set `self.OutboundMoveType` "NewEnumerator3")
                  (`SceneComponent.SetVisibility` (`self.SM_Pallet`) true false)
                  (`/Game/Warehouse/BP_StorageSlot.SetSlotFull` (`self.PalleRack`) (`self.Index`) false)))))
          (:`NewEnumerator3`
            (if (== (mod (`self.Index`) 2) 0)
              (if (<= _relativelocation_y_9 0.0)
                (set `self.OutboundMoveType` "NewEnumerator4"))
              (else
                (set `self.ForkAxis` (0.0 -1.0 0.0))
                (if (>= _relativelocation_y_4 0.0)
                  (set `self.OutboundMoveType` "NewEnumerator4")))))
          (:`NewEnumerator4`
            (if (<= _relativelocation_z_3 (* (`self.Z`) 250))
              (set `self.X` 6)
              (if (>= _relativelocation_x_10 (* (`self.X`) 250))
                (set `self.OutboundMoveType` "NewEnumerator5"))))
          (:`NewEnumerator5`
            (if (>= _relativelocation_y_5 250.0)
              (set `self.OutboundMoveType` "NewEnumerator6")))
          (:`NewEnumerator6`
            (if (<= _relativelocation_y_6 0.0)
              (set `self.OutboundMoveType` "NewEnumerator7")))
          (:`NewEnumerator7`
            (if (<= _relativelocation_z_2 0.0)
              (if (<= _relativelocation_x_6 0.0)
                (set `self.InboundMoveType` "NewEnumerator4")))))))))

(fn `AttachPallet`
  (bind _pallet (`self.Pallet`))
  (if (`KismetSystemLibrary.IsValid` _pallet)
    (`self.K2_AttachToComponent` _pallet (`self.Fork`) "None" "KeepWorld" "KeepWorld" "KeepWorld" false)
    (set `self.Pallet` _pallet)))

(fn `DetachPallet`
  (bind _pallet (`self.Pallet`))
  (if (`KismetSystemLibrary.IsValid` _pallet)
    (`self.K2_DetachFromActor` _pallet "KeepWorld" "KeepWorld" "KeepWorld")))

(fn `InboundDirectionMap`
  (bind _inboundmanager (`self.InboundManager`))
  (bind (_relativelocation_x _relativelocation_y) (`KismetMathLibrary.BreakVector` (`SceneComponent.RelativeLocation` (`self.ForkRoot`))))
  (bind (_relativelocation_x_2 _relativelocation_y_2) (`KismetMathLibrary.BreakVector` (`SceneComponent.RelativeLocation` (`self.ForkRoot`))))
  (bind (_relativelocation_x_3 _relativelocation_y_3) (`KismetMathLibrary.BreakVector` (`SceneComponent.RelativeLocation` (`self.ForkRoot`))))
  (bind _relativelocation_x_4 (`KismetMathLibrary.BreakVector` (`SceneComponent.RelativeLocation` (`self.CraneRoot`))))
  (bind (_relativelocation_x_5 _relativelocation_y_4) (`KismetMathLibrary.BreakVector` (`SceneComponent.RelativeLocation` (`self.ForkRoot`))))
  (bind (_relativelocation_x_6 _relativelocation_y_5) (`KismetMathLibrary.BreakVector` (`SceneComponent.RelativeLocation` (`self.ForkRoot`))))
  (bind (_relativelocation_x_7 _relativelocation_y_6 _relativelocation_z) (`KismetMathLibrary.BreakVector` (`SceneComponent.RelativeLocation` (`self.LiftRoot`))))
  (bind _relativelocation_x_8 (`KismetMathLibrary.BreakVector` (`SceneComponent.RelativeLocation` (`self.CraneRoot`))))
  (bind (_relativelocation_x_9 _relativelocation_y_7 _relativelocation_z_2) (`KismetMathLibrary.BreakVector` (`SceneComponent.RelativeLocation` (`self.LiftRoot`))))
  (bind (_relativelocation_x_10 _relativelocation_y_8) (`KismetMathLibrary.BreakVector` (`SceneComponent.RelativeLocation` (`self.ForkRoot`))))
  (switch `/Game/Warehouse/ENUM/EN_InboundMoveType` (`self.InboundMoveType`)
    (:`NewEnumerator4`
      (set `self.Jobtype` "NewEnumerator0")
      (`/Game/Warehouse/BP_InboudManager.CompleteInbound` _inboundmanager)
      (`/Game/Warehouse/BP_InboudManager.CompleteInboundLog` _inboundmanager))
    (:`NewEnumerator5`
      (if (>= _relativelocation_y_4 250.0)
        (set `self.InboundMoveType` "NewEnumerator6")))
    (:`NewEnumerator6`
      (if (<= _relativelocation_y_5 0.0)
        (set `self.InboundMoveType` "NewEnumerator16")))
    (:`NewEnumerator16`
      (if (>= _relativelocation_x_8 (* (`self.X`) 250))
        (if (>= _relativelocation_z_2 (* (`self.Z`) 250))
          (set `self.InboundMoveType` "NewEnumerator23"))))
    (:`NewEnumerator23`
      (if (== (mod (`self.Index`) 2) 0)
        (if (>= _relativelocation_y 250.0)
          (set `self.InboundMoveType` "NewEnumerator24")
          (`SceneComponent.SetVisibility` (`self.SM_Pallet`) false false)
          (`/Game/Warehouse/BP_StorageSlot.SetSlotFull` (`self.PalleRack`) (`self.Index`) true))
        (else
          (set `self.ForkAxis` (0.0 -1.0 0.0))
          (if (<= _relativelocation_y_2 -250.0)
            (set `self.InboundMoveType` "NewEnumerator24")
            (`SceneComponent.SetVisibility` (`self.SM_Pallet`) false false)
            (`/Game/Warehouse/BP_StorageSlot.SetSlotFull` (`self.PalleRack`) (`self.Index`) true)))))
    (:`NewEnumerator24`
      (if (== (mod (`self.Index`) 2) 0)
        (if (<= _relativelocation_y_8 0.0)
          (set `self.InboundMoveType` "NewEnumerator25"))
        (else
          (set `self.ForkAxis` (0.0 -1.0 0.0))
          (if (>= _relativelocation_y_3 0.0)
            (set `self.InboundMoveType` "NewEnumerator25")))))
    (:`NewEnumerator25`
      (set `self.ForkAxis` (0.0 1.0 0.0))
      (if (<= _relativelocation_z 0.0)
        (if (<= _relativelocation_x_4 0.0)
          (set `self.InboundMoveType` "NewEnumerator4"))))))

(fn `InboundProcess`
  (bind (_find _x _z _index) (`/Game/Warehouse/BP_StorageSlot.FindEmptySlot` (`self.PalleRack`)))
  (if _find
    (set `self.X` _x)
    (bind _output_get (set `self.Z` _z))
    (set `self.Index` _index)
    (`KismetSystemLibrary.PrintString` (`KismetStringLibrary.Conv_IntToString` _output_get))
    (set `self.Jobtype` "NewEnumerator1")
    (set `self.InboundMoveType` "NewEnumerator5")))

(fn `MoveAlongAxis`
  (params (Axis :type "Vector Structure") (Target :type "SceneComponent Object Reference"))
  (`SceneComponent.K2_SetRelativeLocation` Target (`KismetMathLibrary.MakeVector` (`KismetMathLibrary.FClamp` (.x (+ (`SceneComponent.RelativeLocation` Target) (* (`KismetMathLibrary.Normal` Axis 1e-05) (* (`self.Speed`) (`GameplayStatics.GetWorldDeltaSeconds`))))) 0.0 (* (`self.X`) (`self.SlotSize`))) (`KismetMathLibrary.FClamp` (.y (+ (`SceneComponent.RelativeLocation` Target) (* (`KismetMathLibrary.Normal` Axis 1e-05) (* (`self.Speed`) (`GameplayStatics.GetWorldDeltaSeconds`))))) -250.0 250.0) (`KismetMathLibrary.FClamp` (.z (+ (`SceneComponent.RelativeLocation` Target) (* (`KismetMathLibrary.Normal` Axis 1e-05) (* (`self.Speed`) (`GameplayStatics.GetWorldDeltaSeconds`))))) 0.0 (* (`self.Z`) (`self.SlotSize`)))) false false))

(fn `OutboundProcess`
  (bind (_find _x _z _index) (`/Game/Warehouse/BP_StorageSlot.FindOccupiedSlot` (`self.PalleRack`)))
  (if _find
    (set `self.Index` _index)
    (set `self.X` _x)
    (set `self.Z` _z)
    (set `self.Jobtype` "NewEnumerator2")
    (set `self.OutboundMoveType` "NewEnumerator1")))

(fn `SelectOutboundProcess`
  (params (X :type Integer) (Z :type Integer) (Index :type Integer))
  (set `self.X` X)
  (set `self.Z` Z)
  (set `self.Index` Index)
  (set `self.Jobtype` "NewEnumerator2"))

(fn `UserConstructionScript`)