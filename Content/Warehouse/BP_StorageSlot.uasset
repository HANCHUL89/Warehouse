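; Warehouse storage rack actor that tracks which slots in a double-sided X-by-Z grid are full.
; The construction script lays out instanced racks and slot indicators in pairs offset along Y, so index/2 gives the grid cell.
; Lookups return the first empty or occupied slot, while SetSlotFull updates the Full array, ContentRef's count and the indicator's per-instance custom data.
; A text label shows the grid size and faces the camera each tick.
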(event `self.ReceiveBeginPlay`
  (for _index (range (* (* (`self.X`) (`self.Z`)) 2))
    (`KismetArrayLibrary.Array_Set` (`self.Full`) _index false true)
    (`TextRenderComponent.K2_SetText` (`self.TextRender`) (`KismetTextLibrary.Conv_StringToText` (`KismetStringLibrary.Concat_StrStr` (`KismetStringLibrary.Conv_IntToString` (`self.X`)) "X" (`KismetStringLibrary.Conv_IntToString` (`self.Z`)))))))

(event `self.ReceiveTick`
  (params (DeltaSeconds :type "Float (single-precision)"))
  (`SceneComponent.K2_SetWorldRotation` (`self.TextRender`) (`KismetMathLibrary.FindLookAtRotation` (`SceneComponent.K2_GetComponentLocation` (`self.TextRender`)) (`self.K2_GetActorLocation` (`GameplayStatics.GetPlayerCameraManager` 0))) false false))

(fn `FindEmptySlot`
  (returns (Find :type Boolean) (X :type Integer) (Z :type Integer) (Index :type Integer))
  (bind _z (`self.Z`))
  (for _index (range (* (* (`self.X`) (`self.Z`)) 2))
    (if (not (`|GetArrayItem` (`self.Full`) _index))
      (bind _returnvalue (/ _index 2))
      (return true (/ _returnvalue _z) (mod _returnvalue _z) _index)))
  (return false -1 -1 -1))

(fn `FindOccupiedSlot`
  (returns (Find :type Boolean) (X :type Integer) (Z :type Integer) (Index :type Integer))
  (bind _z (`self.Z`))
  (for _index (range (* (* (`self.X`) (`self.Z`)) 2))
    (if (`|GetArrayItem` (`self.Full`) _index)
      (bind _returnvalue (/ _index 2))
      (return true (/ _returnvalue _z) (mod _returnvalue _z) _index)))
  (return false -1 -1 -1))

(fn `GetSlotInfo`
  (params (Index :type Integer))
  (returns (Z :type Integer) (X :type Integer))
  (bind _returnvalue (/ Index 2))
  (bind _z (`self.Z`))
  (return (- (- _z 1) (mod _returnvalue _z)) (- (- (`self.X`) 1) (/ _returnvalue _z))))

(fn `GetSlotWorldLocation`
  (params (X :type Integer) (Z :type Integer))
  (returns (Location :type "Vector Structure"))
  (bind (_returnvalue_x _returnvalue_y _returnvalue_z) (`KismetMathLibrary.BreakVector` (`SceneComponent.K2_GetComponentLocation` (`self.SlotOrigin`))))
  (return (`KismetMathLibrary.MakeVector` (+ (* X (`self.Size`)) _returnvalue_x) _returnvalue_y (+ (* Z (`self.Size`)) _returnvalue_z))))

(fn `SetSlotFull`
  (params (Index :type Integer) (Full :type Boolean))
  (bind _full (`self.Full`))
  (`KismetArrayLibrary.Array_Set` _full Index Full)
  (`/Game/Warehouse/BP_Slot.RefreshCountFromSlot` (`self.ContentRef`) _full)
  (if Full
    (`InstancedStaticMeshComponent.SetCustomDataValue` (`self.SlotIndicators`) Index 0 1.0 false)
    (else
      (`InstancedStaticMeshComponent.SetCustomDataValue` (`self.SlotIndicators`) Index 0 0.0 false))))

(fn `UserConstructionScript`
  (`InstancedStaticMeshComponent.ClearInstances` (`self.SlotIndicators`))
  (for _index (range (* (`self.X`) (`self.Z`)))
    (bind _location (`self.GetSlotWorldLocation` (/ _index (`self.Z`)) (mod _index (`self.Z`))))
    (bind _x (.x _location))
    (bind _y (.y _location))
    (bind _z (.z _location))
    (bind _returnvalue (`KismetMathLibrary.MakeVector` _x (+ _y (`self.GapY`)) _z))
    (`InstancedStaticMeshComponent.AddInstance` (`self.PalletRack`) (`KismetMathLibrary.MakeTransform` _returnvalue (struct) (0.833 1.666 1.23)) true)
    (bind _returnvalue_2 (`KismetMathLibrary.MakeVector` _x (- _y (`self.GapY`)) _z))
    (`InstancedStaticMeshComponent.AddInstance` (`self.PalletRack`) (`KismetMathLibrary.MakeTransform` _returnvalue_2 (struct) (0.833 1.666 1.23)) true)
    (`InstancedStaticMeshComponent.AddInstance` (`self.SlotIndicators`) (`KismetMathLibrary.MakeTransform` (`KismetMathLibrary.MakeVector` (.x _returnvalue) (.y _returnvalue) (+ (.z _returnvalue) 200.0)) (struct) (1.5 0.1 0.1)) true)
    (`InstancedStaticMeshComponent.AddInstance` (`self.SlotIndicators`) (`KismetMathLibrary.MakeTransform` (`KismetMathLibrary.MakeVector` (.x _returnvalue_2) (.y _returnvalue_2) (+ (.z _returnvalue_2) 200.0)) (struct) (1.5 0.1 0.1)) true)))