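; BP_StorageLine is a selectable storage line actor in the warehouse.
; Clicking its Box passes the actor to GM_Warehouse's SelectStorageLine, and an instance flagged DefultLine makes the same call on BeginPlay.
; Every tick its TextRender rotates to face the player camera, acting as a billboard label.
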(event `self.ReceiveTick`
  (params (DeltaSeconds :type "Float (single-precision)"))
  (`SceneComponent.K2_SetWorldRotation` (`self.TextRender`) (`KismetMathLibrary.FindLookAtRotation` (`SceneComponent.K2_GetComponentLocation` (`self.TextRender`)) (`self.K2_GetActorLocation` (`GameplayStatics.GetPlayerCameraManager` 0))) false false))

(event `self.Box.OnClicked`
  (params (TouchedComponent :type "PrimitiveComponent Object Reference") (ButtonPressed :type "Key Structure"))
  (bind _asgm_warehouse (cast `/Game/Warehouse/GM_Warehouse` (`GameplayStatics.GetGameMode`)))
  (`/Game/Warehouse/GM_Warehouse.SelectStorageLine` _asgm_warehouse self))

(event `self.ReceiveBeginPlay`
  (if (`self.DefultLine`)
    (bind _asgm_warehouse (cast `/Game/Warehouse/GM_Warehouse` (`GameplayStatics.GetGameMode`)))
    (`/Game/Warehouse/GM_Warehouse.SelectStorageLine` _asgm_warehouse self)))

(fn `UserConstructionScript`)