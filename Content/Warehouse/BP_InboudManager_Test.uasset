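; Warehouse inbound manager that spawns pallets and hands them to the crane for inbound processing.
; Manual requests queue one pallet, while auto requests reset the queue and add one per empty storage slot.
; A busy flag limits spawning to one pallet at a time, released by CompleteInbound.
; Pallets move to the inbound point, where trigger overlap starts the crane; a text label faces the camera every tick.
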(event `self.InboundTrigger.OnComponentBeginOverlap`
  (params (OverlappedComponent :type "PrimitiveComponent Object Reference") (OtherActor :type "Actor Object Reference") (OtherComp :type "PrimitiveComponent Object Reference") (OtherBodyIndex :type Integer) (bFromSweep :type Boolean) (SweepResult :type "HitResult Structure (by ref)"))
  (cast `/Game/Warehouse/BP_Pallet_Test` OtherActor)
  (`/Game/Warehouse/BP_StackerCrane_Test_02.InboundProcess` (`self.Crane`)))

(event `self.ReceiveTick`
  (params (DeltaSeconds :type "Float (single-precision)"))
  (`SceneComponent.K2_SetWorldRotation` (`self.Txt_Inbound`) (`KismetMathLibrary.FindLookAtRotation` (`SceneComponent.K2_GetComponentLocation` (`self.Txt_Inbound`)) (`self.K2_GetActorLocation` (`GameplayStatics.GetPlayerCameraManager` 0))) false false))

(fn `CompleteInbound`
  (set `self.IsInbounding` false)
  (`self.TrySpawnNextInbound`))

(fn `RequestAutoInbound`
  (set `self.PendingInboundCount` 0)
  (for _index (range 25)
    (if (not (`|GetArrayItem` (`/Game/Warehouse/BP_StorageSlot_Test.Full` (`self.StorageSlot`)) _index))
      (set `self.PendingInboundCount` (+ (`self.PendingInboundCount`) 1))
      (`self.TrySpawnNextInbound`)))
  (if (> (`self.PendingInboundCount`) 0)
    (`self.TrySpawnNextInbound`)))

(fn `RequestInbound`
  (set `self.PendingInboundCount` (+ (`self.PendingInboundCount`) 1))
  (`self.TrySpawnNextInbound`))

(fn `TrySpawnNextInbound`
  (if (`self.IsInbounding`)
    _
    (elif (> (`self.PendingInboundCount`) 0)
      (set `self.IsInbounding` true)
      (set `self.PendingInboundCount` (- (`self.PendingInboundCount`) 1))
      (bind _returnvalue (`|SpawnActorFromClass` "/Game/Warehouse/BP_Pallet_Test.BP_Pallet_Test_C" (`KismetMathLibrary.MakeTransform` (`SceneComponent.K2_GetComponentLocation` (`self.SpawnPoint`))) "Undefined" "MultiplyWithRoot" null null))
      (`/Game/Warehouse/BP_Pallet_Test.MoveToInbound` _returnvalue (`SceneComponent.K2_GetComponentLocation` (`self.InboundPoint`))))))

(fn `UserConstructionScript`)