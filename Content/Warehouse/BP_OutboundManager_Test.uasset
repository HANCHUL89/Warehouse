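; Warehouse outbound manager that queues pallet retrieval jobs for a crane and clears delivered pallets.
; Single and auto (all full slots) requests feed a pending counter, run one at a time via a busy flag released by CompleteOutbound.
; Selected-slot requests bypass the queue, passing grid coordinates to the crane.
; A pallet overlap sends the crane's pallet to the outbound point, then destroys it; Tick turns the label toward the camera.
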(event `self.OutboundTrigger.OnComponentBeginOverlap`
  (params (OverlappedComponent :type "PrimitiveComponent Object Reference") (OtherActor :type "Actor Object Reference") (OtherComp :type "PrimitiveComponent Object Reference") (OtherBodyIndex :type Integer) (bFromSweep :type Boolean) (SweepResult :type "HitResult Structure (by ref)"))
  (cast `/Game/Warehouse/BP_Pallet` OtherActor)
  (`KismetSystemLibrary.Delay` 1.0)
  (`/Game/Warehouse/BP_Pallet_Test.MoveToOutBound` (`/Game/Warehouse/BP_StackerCrane_Test_02.Pallet` (`self.Crane`)) (`SceneComponent.K2_GetComponentLocation` (`self.OutboundPoint`)))
  (`KismetSystemLibrary.Delay` 3.0)
  (`self.K2_DestroyActor` (`/Game/Warehouse/BP_StackerCrane_Test_02.Pallet` (`self.Crane`)))
  (`self.TryNextOutbound`))

(event `self.ReceiveTick`
  (params (DeltaSeconds :type "Float (single-precision)"))
  (`SceneComponent.K2_SetWorldRotation` (`self.Txt_Outbound`) (`KismetMathLibrary.FindLookAtRotation` (`SceneComponent.K2_GetComponentLocation` (`self.Txt_Outbound`)) (`self.K2_GetActorLocation` (`GameplayStatics.GetPlayerCameraManager` 0))) false false))

(fn `CompleteOutbound`
  (set `self.IsOutbounding` false)
  (`self.TryNextOutbound`))

(fn `RequestAutoOutbound`
  (set `self.PendingOutboundCount` 0)
  (for _index (range 25)
    (if (`|GetArrayItem` (`/Game/Warehouse/BP_StorageSlot_Test.Full` (`self.StorageSlot`)) _index)
      (set `self.PendingOutboundCount` (+ (`self.PendingOutboundCount`) 1))
      (`self.TryNextOutbound`)))
  (if (> (`self.PendingOutboundCount`) 0)
    (`self.TryNextOutbound`)))

(fn `RequestOutbound`
  (set `self.PendingOutboundCount` (+ (`self.PendingOutboundCount`) 1))
  (`self.TryNextOutbound`))

(fn `RequestSelectOutbound`
  (params (SlotIndex :type Integer))
  (`/Game/Warehouse/BP_StackerCrane_Test_02.SelectOutboundProcess` (`self.Crane`) (+ (/ SlotIndex 5) 1) (mod SlotIndex 5) SlotIndex))

(fn `TryNextOutbound`
  (if (`self.IsOutbounding`)
    _
    (elif (> (`self.PendingOutboundCount`) 0)
      (set `self.IsOutbounding` true)
      (set `self.PendingOutboundCount` (- (`self.PendingOutboundCount`) 1))
      (`/Game/Warehouse/BP_StackerCrane_Test_02.OutboundProcess` (`self.Crane`)))))

(fn `UserConstructionScript`)