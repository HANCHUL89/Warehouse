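; GM_Warehouse, by its prefix a game mode, sets up the warehouse screen and tracks the selected storage line.
; On BeginPlay it creates and displays WBP_WarehouseUI, enables the mouse cursor for the first player controller and applies the initial StorageLine.
; SelectStorageLine stores the chosen line and, if the widget is valid, pushes it to the UI through UpdateSelectLine.
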(event `self.ReceiveBeginPlay`
  (bind _returnvalue (`|CreateWidget` "/Game/Warehouse/UI/WBP_WarehouseUI.WBP_WarehouseUI_C"))
  (bind _output_get (set `self.WarehousuUI` _returnvalue))
  (`UserWidget.AddToViewport` _output_get 0)
  (set `PlayerController.bShowMouseCursor` true (`GameplayStatics.GetPlayerController` 0))
  (`self.SelectStorageLine` (`self.StorageLine`)))

(fn `SelectStorageLine`
  (params (SelectLine :type "/Game/Warehouse/BP_StorageLine Object Reference"))
  (bind _warehousuui (`self.WarehousuUI`))
  (bind _output_get (set `self.StorageLine` SelectLine))
  (`/Engine/EditorBlueprintResources/StandardMacros.IsValid` _warehousuui
    (:`Is Valid`
      (`/Game/Warehouse/UI/WBP_WarehouseUI.UpdateSelectLine` _warehousuui _output_get))))

(fn `UserConstructionScript`)