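; Warehouse pallet rack test Blueprint that tracks 25 slots as full or empty and directs a crane to slot locations.
; Inbound searches for an empty slot, marks it full, and sends the Crane to a position GetSlotLocation computes from SlotOrigin, five slots per vertical column.
; InitSlots separately builds slot positions from BaseLocation and fills the Full array, but nothing here calls it.
; BeginPlay is empty, and the event graph's Inbound and crane calls are unwired.
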(event `self.ReceiveBeginPlay`)

(fn `FindEmptySlot`
  (returns (SlotNumber :type Integer))
  (for _index (range 25)
    (if (not (`|GetArrayItem` (`self.Full`) _index))
      (return _index)))
  (return -1))

(fn `GetSlotLocation`
  (params (SlotNumber :type Integer))
  (returns (Location :type "Vector Structure"))
  (return (`KismetMathLibrary.MakeVector` (+ (* (/ SlotNumber 5) (`self.GapX`)) (.x (`SceneComponent.K2_GetComponentLocation` (`self.SlotOrigin`)))) (.y (`SceneComponent.K2_GetComponentLocation` (`self.SlotOrigin`))) (+ (* (mod SlotNumber 5) (`self.GapZ`)) (.z (`SceneComponent.K2_GetComponentLocation` (`self.SlotOrigin`)))))))

(fn `Inbound`
  (params (Pallet :type "/Game/Warehouse/BP_Pallet Object Reference"))
  (returns (SlotNumber :type Integer) (Success :type Boolean) (TargetLocation :type "Vector Structure"))
  (bind _slotnumber (`self.FindEmptySlot`))
  (if (>= _slotnumber 0)
    (`self.SetSlotFull` _slotnumber)
    (bind _location (`self.GetSlotLocation` _slotnumber))
    (`/Game/Warehouse/Test/BP_StackerCrane_Test_05.MoveToSlotLocation` (`self.Crane`) _location)
    (return _slotnumber true (0.0 0.0 0.0))
    (else
      (return -1 false (0.0 0.0 0.0)))))

(fn `InitSlots`
  (bind _cols (`self.Cols`))
  (for _index (range 25)
    (set `self.Rows` (/ _index _cols))
    (set `self.Cols` (mod _index _cols))
    (`KismetArrayLibrary.Array_Add` (`self.Array_PalletSlots`) (`KismetMathLibrary.MakeVector` (+ (.x (`self.BaseLocation`)) (* (`self.Cols`) (`self.GapX`))) (.y (`self.BaseLocation`)) (+ (.z (`self.BaseLocation`)) (* (`self.Rows`) (`self.GapZ`)))))
    (`KismetArrayLibrary.Array_Add` (`self.Full`))))

(fn `SetSlotEmpty`
  (params (SlotNumber :type Integer))
  (`KismetArrayLibrary.Array_Set` (`self.Full`) SlotNumber false))

(fn `SetSlotFull`
  (params (SlotNumber :type Integer))
  (`KismetArrayLibrary.Array_Set` (`self.Full`) SlotNumber true))

(fn `UserConstructionScript`)