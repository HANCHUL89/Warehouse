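; Test Blueprint of a warehouse stacker crane that moves nested crane, lift and fork components along X, Z and Y on a 250-unit grid.
; Helper functions step each axis by Speed and delta time, mostly clamped, with Index picking the fork side for inbound drop-off.
; Enum switches sequence inbound and outbound cycles but are unwired, so events only set state.
; The inbound switch lacks a DetachOut case.
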(event `TestMove_F`
  (set `self.X` 3)
  (set `self.Z` 2)
  (set `self.Index` 0)
  (set `self.InboundMoveType` "NewEnumerator0"))

(event `self.ReceiveBeginPlay`
  (set `self.InboundMoveType` "NewEnumerator1"))

(fn `DetachIn_Move`
  (params (DeltaTime :type "Float (double-precision)"))
  (bind (_relativelocation_x _relativelocation_y) (`KismetMathLibrary.BreakVector` (`SceneComponent.RelativeLocation` (`self.ForkRoot`))))
  (bind (_relativelocation_x_2 _relativelocation_y_2 _relativelocation_z) (`KismetMathLibrary.BreakVector` (`SceneComponent.RelativeLocation` (`self.ForkRoot`))))
  (bind (_relativelocation_x_3 _relativelocation_y_3 _relativelocation_z_2) (`KismetMathLibrary.BreakVector` (`SceneComponent.RelativeLocation` (`self.ForkRoot`))))
  (bind _returnvalue (+ (* (* DeltaTime (`self.Speed`)) (`self.DirY`)) _relativelocation_y))
  (if (<= (* (- (`self.TargetY`) _returnvalue) (`self.DirY`)) 0.0)
    (`SceneComponent.K2_SetRelativeLocation` (`self.ForkRoot`) (`KismetMathLibrary.MakeVector` _relativelocation_x_3 (`self.TargetY`) _relativelocation_z_2) false false)
    (else
      (`SceneComponent.K2_SetRelativeLocation` (`self.ForkRoot`) (`KismetMathLibrary.MakeVector` _relativelocation_x_2 _returnvalue _relativelocation_z) false false))))

(fn `DetachIn_Start`
  (bind (_relativelocation_x _relativelocation_y) (`KismetMathLibrary.BreakVector` (`SceneComponent.RelativeLocation` (`self.ForkRoot`))))
  (set `self.TargetY` (`KismetMathLibrary.SelectFloat` 250.0 -250.0 (>= (`self.Index`) 9)))
  (set `self.DirY` (`KismetMathLibrary.SelectFloat` 1.0 -1.0 (>= (- (`self.TargetY`) _relativelocation_y) 0.0))))

(fn `MoveAlongAxis`
  (params (Axis :type "Vector Structure"))
  (`SceneComponent.K2_SetRelativeLocation` (`self.ForkRoot`) (+ (`SceneComponent.RelativeLocation` (`self.ForkRoot`)) (* (`KismetMathLibrary.Normal` Axis) (* (`self.Speed`) (`GameplayStatics.GetWorldDeltaSeconds`)))) false false))

(fn `MoveX_Left`
  (params (DeltaTime :type "Float (double-precision)"))
  (bind (_relativelocation_x _relativelocation_y _relativelocation_z) (`KismetMathLibrary.BreakVector` (`SceneComponent.RelativeLocation` (`self.CraneRoot`))))
  (`SceneComponent.K2_SetRelativeLocation` (`self.CraneRoot`) (`KismetMathLibrary.MakeVector` (`KismetMathLibrary.FClamp` (+ _relativelocation_x (* DeltaTime (`self.Speed`))) 0.0 (`KismetMathLibrary.Conv_IntToDouble` (* (`self.X`) 250))) _relativelocation_y _relativelocation_z) false false))

(fn `MoveX_Right`
  (params (DeltaTime :type "Float (double-precision)"))
  (bind (_relativelocation_x _relativelocation_y _relativelocation_z) (`KismetMathLibrary.BreakVector` (`SceneComponent.RelativeLocation` (`self.CraneRoot`))))
  (`SceneComponent.K2_SetRelativeLocation` (`self.CraneRoot`) (`KismetMathLibrary.MakeVector` (- _relativelocation_x (* DeltaTime (`self.Speed`))) _relativelocation_y _relativelocation_z) false false))

(fn `MoveY_Back`
  (params (DeltaTime :type "Float (double-precision)"))
  (bind (_relativelocation_x _relativelocation_y _relativelocation_z) (`KismetMathLibrary.BreakVector` (`SceneComponent.RelativeLocation` (`self.ForkRoot`))))
  (`SceneComponent.K2_SetRelativeLocation` (`self.ForkRoot`) (`KismetMathLibrary.MakeVector` _relativelocation_x (`KismetMathLibrary.FClamp` (- _relativelocation_y (* DeltaTime (`self.Speed`))) 0.0 250.0) _relativelocation_z) false false))

(fn `MoveY_Fwd`
  (params (DeltaTime :type "Float (double-precision)"))
  (bind (_relativelocation_x _relativelocation_y _relativelocation_z) (`KismetMathLibrary.BreakVector` (`SceneComponent.RelativeLocation` (`self.ForkRoot`))))
  (`SceneComponent.K2_SetRelativeLocation` (`self.ForkRoot`) (`KismetMathLibrary.MakeVector` _relativelocation_x (`KismetMathLibrary.FClamp` (+ _relativelocation_y (* DeltaTime (`self.Speed`))) 0.0 250.0) _relativelocation_z) false false))

(fn `MoveZ_Down`
  (params (DeltaTime :type "Float (double-precision)"))
  (bind (_relativelocation_x _relativelocation_y _relativelocation_z) (`KismetMathLibrary.BreakVector` (`SceneComponent.RelativeLocation` (`self.LiftRoot`))))
  (`SceneComponent.K2_SetRelativeLocation` (`self.LiftRoot`) (`KismetMathLibrary.MakeVector` _relativelocation_x _relativelocation_y (`KismetMathLibrary.FClamp` (- _relativelocation_z (* DeltaTime (`self.Speed`))) 0.0 (`KismetMathLibrary.Conv_IntToDouble` (* (`self.Z`) 250)))) false false))

(fn `MoveZ_Up`
  (params (DeltaTime :type "Float (double-precision)"))
  (bind (_relativelocation_x _relativelocation_y _relativelocation_z) (`KismetMathLibrary.BreakVector` (`SceneComponent.RelativeLocation` (`self.LiftRoot`))))
  (`SceneComponent.K2_SetRelativeLocation` (`self.LiftRoot`) (`KismetMathLibrary.MakeVector` _relativelocation_x _relativelocation_y (`KismetMathLibrary.FClamp` (+ _relativelocation_z (* DeltaTime (`self.Speed`))) 0.0 (`KismetMathLibrary.Conv_IntToDouble` (* (`self.Z`) 250)))) false false))

(fn `UserConstructionScript`)