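; BP_Slot is a warehouse storage slot that displays its filled positions as instanced static meshes.
; RefreshCountFromSlot clears the HISM, then adds an instance for each true entry in a boolean array, keeping gaps for empty ones.
; Positions pack two across Y, stack StorageSlot.Z high, then advance along X.
; RefreshCount marks the first Count entries full and rebuilds; its Construction Script call is disconnected.
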(event `refreshcount`
  (for _index (range (`self.Count`))
    (`KismetArrayLibrary.Array_Set` (`self.TempFullArray`) _index true true))
  (`self.RefreshCountFromSlot` (`self.TempFullArray`)))

(event `RefreshCountFromSlot`
  (params (Full :type "Array of Boolean"))
  (bind _returnvalue (* (`/Game/Warehouse/BP_StorageSlot.Z` (`self.StorageSlot`)) 2))
  (`InstancedStaticMeshComponent.ClearInstances` (`self.HierarchicalInstancedStaticMesh`))
  (for _index (range (`KismetArrayLibrary.Array_Length` Full))
    (if (`|GetArrayItem` Full _index)
      (`InstancedStaticMeshComponent.AddInstance` (`self.HierarchicalInstancedStaticMesh`) (`KismetMathLibrary.MakeTransform` (`KismetMathLibrary.MakeVector` (* (`KismetMathLibrary.Conv_IntToDouble` (/ _index _returnvalue)) (`self.XDistance`)) (* (`KismetMathLibrary.Conv_IntToDouble` (mod _index 2)) (`self.YDistance`)) (* (`KismetMathLibrary.Conv_IntToDouble` (/ (mod _index _returnvalue) 2)) (`self.ZDistance`)))) false))))

(fn `UserConstructionScript`)