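; Warehouse inbound station manager that spawns pallets, sends them to the inbound point and starts the crane's inbound process when one overlaps the trigger.
; Manual requests add one to a pending count, while auto requests reset it and count every empty storage slot.
; An IsInbounding flag serializes spawning; CompleteInbound clears it, decrements the count, spawns the next pallet or logs completion to the UI.
; Its text label turns toward the camera every tick.
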(event `self.InboundTrigger.OnComponentBeginOverlap`
  (params (OverlappedComponent :type "PrimitiveComponent Object Reference") (OtherActor :type "Actor Object Reference") (OtherComp :type "PrimitiveComponent Object Reference") (OtherBodyIndex :type Integer) (bFromSweep :type Boolean) (SweepResult :type "HitResult Structure (by ref)"))
  (cast `/Game/Warehouse/BP_Pallet` OtherActor)
  (`/Game/Warehouse/BP_StackerCrane.InboundProcess` (`self.Crane`)))

(event `self.ReceiveTick`
  (params (DeltaSeconds :type "Float (single-precision)"))
  (`SceneComponent.K2_SetWorldRotation` (`self.Txt_Inbound`) (`KismetMathLibrary.FindLookAtRotation` (`SceneComponent.K2_GetComponentLocation` (`self.Txt_Inbound`)) (`self.K2_GetActorLocation` (`GameplayStatics.GetPlayerCameraManager` 0))) false false))

(fn `CompleteInbound`
  (set `self.IsInbounding` false)
  (if (> (`self.PendingInboundCount`) 0)
    (set `self.PendingInboundCount` (- (`self.PendingInboundCount`) 1))
    (`self.TrySpawnNextInbound`)
    (if (`self.IsInbounding`)
      _
      (elif (<= (`self.PendingInboundCount`) 0)
        (bind _asgm_warehouse (cast `/Game/Warehouse/GM_Warehouse` (`GameplayStatics.GetGameMode`)))
        (`/Game/Warehouse/UI/WBP_WarehouseUI.CompleteInboundLog` (`/Game/Warehouse/GM_Warehouse.WarehousuUI` _asgm_warehouse) (`self.StorageLine`))))))

(fn `RequestAutoInbound`
  (bind _storageslot (`self.StorageSlot`))
  (bind _asgm_warehouse (cast `/Game/Warehouse/GM_Warehouse` (`GameplayStatics.GetGameMode`)))
  (set `/Game/Warehouse/BP_StackerCrane.CraneStatus` "크레인 상태 : 입고 작업" (`/Game/Warehouse/BP_StorageLine.Crane` (`/Game/Warehouse/GM_Warehouse.StorageLine` _asgm_warehouse)))
  (`/Game/Warehouse/UI/WBP_WarehouseUI.AddLogEntry` (`/Game/Warehouse/GM_Warehouse.WarehousuUI` _asgm_warehouse) "\"자동 입고 요청 등록\"")
  (set `self.PendingInboundCount` 0)
  (for _index (range (* (* (`/Game/Warehouse/BP_StorageSlot.X` _storageslot) (`/Game/Warehouse/BP_StorageSlot.Z` _storageslot)) 2))
    (if (not (`|GetArrayItem` (`/Game/Warehouse/BP_StorageSlot.Full` _storageslot) _index))
      (set `self.PendingInboundCount` (+ (`self.PendingInboundCount`) 1))
      (`self.TrySpawnNextInbound`)))
  (if (> (`self.PendingInboundCount`) 0)
    (`self.TrySpawnNextInbound`)))

(fn `RequestInbound`
  (set `self.PendingInboundCount` (+ (`self.PendingInboundCount`) 1))
  (`self.TrySpawnNextInbound`)
  (bind _asgm_warehouse (cast `/Game/Warehouse/GM_Warehouse` (`GameplayStatics.GetGameMode`)))
  (set `/Game/Warehouse/BP_StackerCrane.CraneStatus` "크레인 상태 : 입고 작업" (`/Game/Warehouse/BP_StorageLine.Crane` (`/Game/Warehouse/GM_Warehouse.StorageLine` _asgm_warehouse)))
  (`/Game/Warehouse/UI/WBP_WarehouseUI.AddLogEntry` (`/Game/Warehouse/GM_Warehouse.WarehousuUI` _asgm_warehouse) "\"수동 입고 요청 등록\""))

(fn `TrySpawnNextInbound`
  (if (`self.IsInbounding`)
    _
    (elif (> (`self.PendingInboundCount`) 0)
      (set `self.IsInbounding` true)
      (bind _returnvalue (`|SpawnActorFromClass` "/Game/Warehouse/BP_Pallet.BP_Pallet_C" (`KismetMathLibrary.MakeTransform` (`SceneComponent.K2_GetComponentLocation` (`self.SpawnPoint`))) "Undefined" "MultiplyWithRoot" null null))
      (`/Game/Warehouse/BP_Pallet.MoveToInbound` _returnvalue (`SceneComponent.K2_GetComponentLocation` (`self.InboundPoint`))))))

(fn `UserConstructionScript`)